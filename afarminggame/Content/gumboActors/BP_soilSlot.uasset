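; Soil plot actor that plants a crop based on the player character's selected Seeds value.
; The plantSeed event and the Box component's hit event both run the same switch on that value.
; Every crop case spawns the same BP_basePlant slightly offset in Y from the slot, differing only in the debug message.
; Phone and Watering Can only print a message, and the slot has no occupancy check.
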(event `plantSeed`
  (bind (_returnvalue_x _returnvalue_y _returnvalue_z) (`KismetMathLibrary.BreakVector` (`self.K2_GetActorLocation`)))
  (bind (_returnvalue_x_2 _returnvalue_y_2 _returnvalue_z_2) (`KismetMathLibrary.BreakVector` (`self.K2_GetActorLocation`)))
  (bind (_returnvalue_x_3 _returnvalue_y_3 _returnvalue_z_3) (`KismetMathLibrary.BreakVector` (`self.K2_GetActorLocation`)))
  (bind (_returnvalue_x_4 _returnvalue_y_4 _returnvalue_z_4) (`KismetMathLibrary.BreakVector` (`self.K2_GetActorLocation`)))
  (bind (_returnvalue_x_5 _returnvalue_y_5 _returnvalue_z_5) (`KismetMathLibrary.BreakVector` (`self.K2_GetActorLocation`)))
  (bind (_returnvalue_x_6 _returnvalue_y_6 _returnvalue_z_6) (`KismetMathLibrary.BreakVector` (`self.K2_GetActorLocation`)))
  (bind (_returnvalue_x_7 _returnvalue_y_7 _returnvalue_z_7) (`KismetMathLibrary.BreakVector` (`self.K2_GetActorLocation`)))
  (bind (_returnvalue_x_8 _returnvalue_y_8 _returnvalue_z_8) (`KismetMathLibrary.BreakVector` (`self.K2_GetActorLocation`)))
  (bind _asbp_first_person_character (cast `/Game/FirstPerson/Blueprints/BP_FirstPersonCharacter` (`GameplayStatics.GetPlayerCharacter` 0) :!label _label))
  (switch `/Game/gumboActors/Items+seeds` (`/Game/FirstPerson/Blueprints/BP_FirstPersonCharacter.Seeds` _asbp_first_person_character)
    (:`NewEnumerator8`
      (`KismetSystemLibrary.PrintString` "you cant use phone (1)"))
    (:`NewEnumerator9`
      (`KismetSystemLibrary.PrintString` "using watering can (2)"))
    (:`NewEnumerator0`
      (`|SpawnActorFromClass` "/Game/gumboActors/plantBPs/BP_basePlant.BP_basePlant_C" (`KismetMathLibrary.MakeTransform` (`KismetMathLibrary.MakeVector` _returnvalue_x_3 (+ _returnvalue_y_3 10.0) _returnvalue_z_3)) "Undefined" "MultiplyWithRoot" null null)
      (`KismetSystemLibrary.PrintString` "carrot spawned"))
    (:`NewEnumerator1`
      (`|SpawnActorFromClass` "/Game/gumboActors/plantBPs/BP_basePlant.BP_basePlant_C" (`KismetMathLibrary.MakeTransform` (`KismetMathLibrary.MakeVector` _returnvalue_x_4 (+ _returnvalue_y_4 10.0) _returnvalue_z_4)) "Undefined" "MultiplyWithRoot" null null)
      (`KismetSystemLibrary.PrintString` "potato spawned"))
    (:`NewEnumerator2`
      (`|SpawnActorFromClass` "/Game/gumboActors/plantBPs/BP_basePlant.BP_basePlant_C" (`KismetMathLibrary.MakeTransform` (`KismetMathLibrary.MakeVector` _returnvalue_x_5 (+ _returnvalue_y_5 10.0) _returnvalue_z_5)) "Undefined" "MultiplyWithRoot" null null)
      (`KismetSystemLibrary.PrintString` "onion spawned"))
    (:`NewEnumerator3`
      (`|SpawnActorFromClass` "/Game/gumboActors/plantBPs/BP_basePlant.BP_basePlant_C" (`KismetMathLibrary.MakeTransform` (`KismetMathLibrary.MakeVector` _returnvalue_x (+ _returnvalue_y 10.0) _returnvalue_z)) "Undefined" "MultiplyWithRoot" null null)
      (`KismetSystemLibrary.PrintString` "corn spawned"))
    (:`NewEnumerator4`
      (`|SpawnActorFromClass` "/Game/gumboActors/plantBPs/BP_basePlant.BP_basePlant_C" (`KismetMathLibrary.MakeTransform` (`KismetMathLibrary.MakeVector` _returnvalue_x_2 (+ _returnvalue_y_2 10.0) _returnvalue_z_2)) "Undefined" "MultiplyWithRoot" null null)
      (`KismetSystemLibrary.PrintString` "tomato spawned"))
    (:`NewEnumerator5`
      (`|SpawnActorFromClass` "/Game/gumboActors/plantBPs/BP_basePlant.BP_basePlant_C" (`KismetMathLibrary.MakeTransform` (`KismetMathLibrary.MakeVector` _returnvalue_x_6 (+ _returnvalue_y_6 10.0) _returnvalue_z_6)) "Undefined" "MultiplyWithRoot" null null)
      (`KismetSystemLibrary.PrintString` "pumpkin spawned"))
    (:`NewEnumerator6`
      (`|SpawnActorFromClass` "/Game/gumboActors/plantBPs/BP_basePlant.BP_basePlant_C" (`KismetMathLibrary.MakeTransform` (`KismetMathLibrary.MakeVector` _returnvalue_x_8 (+ _returnvalue_y_8 10.0) _returnvalue_z_8)) "Undefined" "MultiplyWithRoot" null null)
      (`KismetSystemLibrary.PrintString` "watermelon spawned"))
    (:`NewEnumerator7`
      (`|SpawnActorFromClass` "/Game/gumboActors/plantBPs/BP_basePlant.BP_basePlant_C" (`KismetMathLibrary.MakeTransform` (`KismetMathLibrary.MakeVector` _returnvalue_x_7 (+ _returnvalue_y_7 10.0) _returnvalue_z_7)) "Undefined" "MultiplyWithRoot" null null)
      (`KismetSystemLibrary.PrintString` "grapes spawned"))))

(event `self.Box.OnComponentHit`
  (params (HitComponent :type "PrimitiveComponent Object Reference") (OtherActor :type "Actor Object Reference") (OtherComp :type "PrimitiveComponent Object Reference") (NormalImpulse :type "Vector Structure") (Hit :type "HitResult Structure (by ref)"))
  (goto _label))

(fn `UserConstructionScript`)