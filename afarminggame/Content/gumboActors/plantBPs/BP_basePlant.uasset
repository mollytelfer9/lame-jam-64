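; Base plant actor for a time-skip farming game, growing in its owning soil slot and turning in yaw to face the player.
; Aging subtracts the TimeSkipManager's skipped years if the soil is watered, updating labels or triggering growth; unwatered plants are destroyed.
; Harvesting reprices the crop through MarketManager even before the grown check.
; Grown plants then pay the player, free the slot, check for a win and destroy themselves.
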(event `self.ReceiveTick`
  (params (DeltaSeconds :type "Float (single-precision)"))
  (bind (_returnvalue_roll _returnvalue_pitch _returnvalue_yaw) (`KismetMathLibrary.BreakRotator` (`KismetMathLibrary.FindLookAtRotation` (`self.K2_GetActorLocation`) (`self.K2_GetActorLocation` (`GameplayStatics.GetPlayerCharacter` 0)))))
  ; face player
  (`self.K2_SetActorRotation` (`KismetMathLibrary.RInterpTo` (`self.K2_GetActorRotation`) (`KismetMathLibrary.MakeRotator` 0.0 0.0 _returnvalue_yaw) (`GameplayStatics.GetWorldDeltaSeconds`))))

(event `self.ReceiveBeginPlay`
  (bind _returnvalue (`GameplayStatics.GetActorOfClass` "/Game/timeSkip/timeSkipManager.timeSkipManager_C"))
  (set `self.timeManagerRef` _returnvalue)
  (bind _returnvalue_2 (`GameplayStatics.GetActorOfClass` "/Game/FirstPerson/Blueprints/BP_FirstPersonCharacter.BP_FirstPersonCharacter_C"))
  (set `self.playerRef` _returnvalue_2)
  (`self.updateText`)
  (bind _asbp_soil_slot (cast `/Game/gumboActors/BP_soilSlot` (`self.GetOwner`)))
  (set `self.soilRef` _asbp_soil_slot))

(event `plantAge`
  (`KismetSystemLibrary.PrintString` "plant aged")
  (if (`/Game/gumboActors/BP_soilSlot.isWatered` (`self.soilRef`))
    (set `self.yearsLeft` (- (`self.yearsLeft`) (`/Game/timeSkip/timeSkipManager.yearsToSkip` (`self.timeManagerRef`))))
    (if (<= (`self.yearsLeft`) 0.0)
      (`self.plantGrow`)
      (else
        (`self.updateText`)))
    (else
      (set `/Game/gumboActors/BP_soilSlot.hasSeeds` false (`self.soilRef`))
      (`self.K2_DestroyActor`))))

(event `plantGrow`
  (`SceneComponent.ToggleVisibility` (`self.PaperSprite`) false)
  (`SceneComponent.ToggleVisibility` (`self.plantType`) false)
  (`SceneComponent.ToggleVisibility` (`self.yearsLeftText`) false)
  (`KismetSystemLibrary.PrintString` "plant grow")
  (set `self.isGrown` true)
  (bind _returnvalue (`GameplayStatics.GetActorOfClass` "/Game/gumboActors/audioManager.audioManager_C"))
  (`/Game/gumboActors/audioManager.plantGrowAudio` _returnvalue))

(event `harvestPlant`
  (bind _playerref (`self.playerRef`))
  (bind _playerref_2 (`self.playerRef`))
  (bind _returnvalue (`GameplayStatics.GetActorOfClass` "/Game/menusUI/marketManager.marketManager_C"))
  (bind _newplantvalue (`/Game/menusUI/marketManager.decreaseSellValue` _returnvalue (`self.plantName`) (`self.plantValue`)))
  (bind _output_get (set `self.plantValue` (`KismetMathLibrary.Conv_IntToDouble` (`KismetMathLibrary.Round` _newplantvalue))))
  (if (`self.isGrown`)
    (set `/Game/FirstPerson/Blueprints/BP_FirstPersonCharacter.moneyEarned` (+ (`/Game/FirstPerson/Blueprints/BP_FirstPersonCharacter.moneyEarned` _playerref) _output_get) _playerref_2)
    (`/Engine/EditorBlueprintResources/StandardMacros.IncrementFloat` (`/Game/FirstPerson/Blueprints/BP_FirstPersonCharacter.totalCropsSold` _playerref)
      (:`  `
        (bind _asbp_soil_slot (cast `/Game/gumboActors/BP_soilSlot` (`self.GetOwner`)))
        (set `/Game/gumboActors/BP_soilSlot.hasSeeds` false _asbp_soil_slot)
        (`/Game/gumboActors/BP_soilSlot.updateSoilSprite` _asbp_soil_slot)
        (`GameplayStatics.PlaySound2D` "/Game/gumboActors/audio/plantHarvested.plantHarvested" 1.0 1.0 0.0 null null)
        (`/Game/FirstPerson/Blueprints/BP_FirstPersonCharacter.checkWin` _playerref_2)
        (`self.K2_DestroyActor`)))))

(fn `UserConstructionScript`)