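; BP_soilSlot is a farm soil plot that the player can water or plant with one crop, shown as a Paper2D sprite yawed toward the player each tick.
; plantSeed switches on the player's selected item, either watering the plot or spawning the matching crop actor at SpawnAboveSoil and using up a seed.
; Successful actions play a sound, spend stamina, refresh the HUD and set the sprite from the IsWatered and HasSeeds flags.
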(event `self.ReceiveTick`
  (params (DeltaSeconds :type "Float (single-precision)"))
  (bind (_returnvalue_roll _returnvalue_pitch _returnvalue_yaw) (`KismetMathLibrary.BreakRotator` (`KismetMathLibrary.FindLookAtRotation` (`self.K2_GetActorLocation`) (`self.K2_GetActorLocation` (`GameplayStatics.GetPlayerCharacter` 0)))))
  ; face player
  (`self.K2_SetActorRotation` (`KismetMathLibrary.RInterpTo` (`self.K2_GetActorRotation`) (`KismetMathLibrary.MakeRotator` 0.0 0.0 _returnvalue_yaw) (`GameplayStatics.GetWorldDeltaSeconds`))))

(event `self.ReceiveBeginPlay`
  (bind _asbp_first_person_character (cast `/Game/FirstPerson/Blueprints/BP_FirstPersonCharacter` (`GameplayStatics.GetPlayerCharacter` 0)))
  (set `self.playerRef` _asbp_first_person_character))

(event `plantSeed`
  (bind (_returnvalue_x _returnvalue _returnvalue_z) (`self.spawnAboveSoil`))
  (bind (_returnvalue_x_2 _returnvalue_2 _returnvalue_z_2) (`self.spawnAboveSoil`))
  (bind (_returnvalue_x_3 _returnvalue_3 _returnvalue_z_3) (`self.spawnAboveSoil`))
  (bind (_returnvalue_x_4 _returnvalue_4 _returnvalue_z_4) (`self.spawnAboveSoil`))
  (bind (_returnvalue_x_5 _returnvalue_5 _returnvalue_z_5) (`self.spawnAboveSoil`))
  (bind (_returnvalue_x_6 _returnvalue_6 _returnvalue_z_6) (`self.spawnAboveSoil`))
  (bind (_returnvalue_x_7 _returnvalue_7 _returnvalue_z_7) (`self.spawnAboveSoil`))
  (bind (_returnvalue_x_8 _returnvalue_8 _returnvalue_z_8) (`self.spawnAboveSoil`))
  (bind _playerref (`self.playerRef`))
  (switch `/Game/gumboActors/Items+seeds` (`/Game/FirstPerson/Blueprints/BP_FirstPersonCharacter.Seeds` (`self.playerRef`))
    (:`NewEnumerator8`)
    (:`NewEnumerator9`
      (if (not (`self.isWatered`))
        (set `self.isWatered` true)
        (`self.updateSoilSprite`)
        (`GameplayStatics.PlaySound2D` "/Game/gumboActors/audio/wateringCan.wateringCan" 1.0 1.0 0.0 null null)
        (set `/Game/FirstPerson/Blueprints/BP_FirstPersonCharacter.Stamina` (- (`/Game/FirstPerson/Blueprints/BP_FirstPersonCharacter.Stamina` _playerref) (`/Game/FirstPerson/Blueprints/BP_FirstPersonCharacter.staminaCost` _playerref)) _playerref :!label _label)
        (`/Game/menusUI/UI_playerHUD.updateStacks` (`/Game/FirstPerson/Blueprints/BP_FirstPersonCharacter.hudRef` _playerref))))
    (:`NewEnumerator0`
      (if (and (> (`/Game/FirstPerson/Blueprints/BP_FirstPersonCharacter.carrotSeeds` (`self.playerRef`)) 0.0) (not (`self.hasSeeds`)))
        (`|SpawnActorFromClass` "/Game/gumboActors/plantBPs/BP_Carrot.BP_Carrot_C" (`KismetMathLibrary.MakeTransform` (`KismetMathLibrary.MakeVector` _returnvalue_x_2 _returnvalue_2 _returnvalue_z_2)) "Undefined" "MultiplyWithRoot" self null)
        (bind _result (`/Engine/EditorBlueprintResources/StandardMacros.DecrementFloat` (`/Game/FirstPerson/Blueprints/BP_FirstPersonCharacter.carrotSeeds` (`self.playerRef`)))
          (:`  `
            (set `/Game/FirstPerson/Blueprints/BP_FirstPersonCharacter.carrotSeeds` _result (`self.playerRef`))
            (set `self.hasSeeds` true :!label _label_2)
            (`self.updateSoilSprite`)
            (`GameplayStatics.PlaySound2D` "/Game/gumboActors/audio/plantSeed.plantSeed" 1.0 1.0 0.0 null null)
            (goto _label)))))
    (:`NewEnumerator1`
      (if (and (> (`/Game/FirstPerson/Blueprints/BP_FirstPersonCharacter.potatoSeeds` (`self.playerRef`)) 0.0) (not (`self.hasSeeds`)))
        (`|SpawnActorFromClass` "/Game/gumboActors/plantBPs/BP_Potato.BP_Potato_C" (`KismetMathLibrary.MakeTransform` (`KismetMathLibrary.MakeVector` _returnvalue_x_3 _returnvalue_3 _returnvalue_z_3)) "Undefined" "MultiplyWithRoot" self null)
        (bind _result_2 (`/Engine/EditorBlueprintResources/StandardMacros.DecrementFloat` (`/Game/FirstPerson/Blueprints/BP_FirstPersonCharacter.potatoSeeds` (`self.playerRef`)))
          (:`  `
            (set `/Game/FirstPerson/Blueprints/BP_FirstPersonCharacter.potatoSeeds` _result_2 (`self.playerRef`))
            (goto _label_2)))))
    (:`NewEnumerator2`
      (if (and (> (`/Game/FirstPerson/Blueprints/BP_FirstPersonCharacter.onionSeeds` (`self.playerRef`)) 0.0) (not (`self.hasSeeds`)))
        (`|SpawnActorFromClass` "/Game/gumboActors/plantBPs/BP_Onion.BP_Onion_C" (`KismetMathLibrary.MakeTransform` (`KismetMathLibrary.MakeVector` _returnvalue_x_4 _returnvalue_4 _returnvalue_z_4)) "Undefined" "MultiplyWithRoot" self null)
        (bind _result_3 (`/Engine/EditorBlueprintResources/StandardMacros.DecrementFloat` (`/Game/FirstPerson/Blueprints/BP_FirstPersonCharacter.onionSeeds` (`self.playerRef`)))
          (:`  `
            (set `/Game/FirstPerson/Blueprints/BP_FirstPersonCharacter.onionSeeds` _result_3 (`self.playerRef`))
            (goto _label_2)))))
    (:`NewEnumerator3`
      (if (and (> (`/Game/FirstPerson/Blueprints/BP_FirstPersonCharacter.cornSeeds` (`self.playerRef`)) 0.0) (not (`self.hasSeeds`)))
        (`|SpawnActorFromClass` "/Game/gumboActors/plantBPs/BP_Corn.BP_Corn_C" (`KismetMathLibrary.MakeTransform` (`KismetMathLibrary.MakeVector` _returnvalue_x_5 _returnvalue_5 _returnvalue_z_5)) "Undefined" "MultiplyWithRoot" self null)
        (bind _result_4 (`/Engine/EditorBlueprintResources/StandardMacros.DecrementFloat` (`/Game/FirstPerson/Blueprints/BP_FirstPersonCharacter.cornSeeds` (`self.playerRef`)))
          (:`  `
            (set `/Game/FirstPerson/Blueprints/BP_FirstPersonCharacter.cornSeeds` _result_4 (`self.playerRef`))
            (goto _label_2)))))
    (:`NewEnumerator4`
      (if (and (> (`/Game/FirstPerson/Blueprints/BP_FirstPersonCharacter.tomatoSeeds` (`self.playerRef`)) 0.0) (not (`self.hasSeeds`)))
        (`|SpawnActorFromClass` "/Game/gumboActors/plantBPs/BP_Tomato.BP_Tomato_C" (`KismetMathLibrary.MakeTransform` (`KismetMathLibrary.MakeVector` _returnvalue_x_6 _returnvalue_6 _returnvalue_z_6)) "Undefined" "MultiplyWithRoot" self null)
        (bind _result_5 (`/Engine/EditorBlueprintResources/StandardMacros.DecrementFloat` (`/Game/FirstPerson/Blueprints/BP_FirstPersonCharacter.tomatoSeeds` (`self.playerRef`)))
          (:`  `
            (set `/Game/FirstPerson/Blueprints/BP_FirstPersonCharacter.tomatoSeeds` _result_5 (`self.playerRef`))
            (goto _label_2)))))
    (:`NewEnumerator5`
      (if (and (> (`/Game/FirstPerson/Blueprints/BP_FirstPersonCharacter.pumpkinSeeds` (`self.playerRef`)) 0.0) (not (`self.hasSeeds`)))
        (`|SpawnActorFromClass` "/Game/gumboActors/plantBPs/BP_Pumpkin.BP_Pumpkin_C" (`KismetMathLibrary.MakeTransform` (`KismetMathLibrary.MakeVector` _returnvalue_x_7 _returnvalue_7 _returnvalue_z_7)) "Undefined" "MultiplyWithRoot" self null)
        (bind _result_6 (`/Engine/EditorBlueprintResources/StandardMacros.DecrementFloat` (`/Game/FirstPerson/Blueprints/BP_FirstPersonCharacter.pumpkinSeeds` (`self.playerRef`)))
          (:`  `
            (set `/Game/FirstPerson/Blueprints/BP_FirstPersonCharacter.pumpkinSeeds` _result_6 (`self.playerRef`))
            (goto _label_2)))))
    (:`NewEnumerator6`
      (if (and (> (`/Game/FirstPerson/Blueprints/BP_FirstPersonCharacter.watermelonSeeds` (`self.playerRef`)) 0.0) (not (`self.hasSeeds`)))
        (`|SpawnActorFromClass` "/Game/gumboActors/plantBPs/BP_Watermelon.BP_Watermelon_C" (`KismetMathLibrary.MakeTransform` (`KismetMathLibrary.MakeVector` _returnvalue_x_8 _returnvalue_8 _returnvalue_z_8)) "Undefined" "MultiplyWithRoot" self null)
        (bind _result_7 (`/Engine/EditorBlueprintResources/StandardMacros.DecrementFloat` (`/Game/FirstPerson/Blueprints/BP_FirstPersonCharacter.watermelonSeeds` (`self.playerRef`)))
          (:`  `
            (set `/Game/FirstPerson/Blueprints/BP_FirstPersonCharacter.watermelonSeeds` _result_7 (`self.playerRef`))
            (goto _label_2)))))
    (:`NewEnumerator7`
      (if (and (> (`/Game/FirstPerson/Blueprints/BP_FirstPersonCharacter.grapeSeeds` (`self.playerRef`)) 0.0) (not (`self.hasSeeds`)))
        (`|SpawnActorFromClass` "/Game/gumboActors/plantBPs/BP_Grapes.BP_Grapes_C" (`KismetMathLibrary.MakeTransform` (`KismetMathLibrary.MakeVector` _returnvalue_x _returnvalue _returnvalue_z)) "Undefined" "MultiplyWithRoot" self null)
        (bind _result_8 (`/Engine/EditorBlueprintResources/StandardMacros.DecrementFloat` (`/Game/FirstPerson/Blueprints/BP_FirstPersonCharacter.grapeSeeds` (`self.playerRef`)))
          (:`  `
            (set `/Game/FirstPerson/Blueprints/BP_FirstPersonCharacter.grapeSeeds` _result_8 (`self.playerRef`))
            (goto _label_2)))))))

(event `updateSoilSprite`
  (if (`self.isWatered`)
    (if (`self.hasSeeds`)
      (`PaperSpriteComponent.SetSprite` (`self.PaperSprite`) "/Game/gumboActors/soilSprites/wetSoilPlanted_Sprite.wetSoilPlanted_Sprite")
      (else
        (`PaperSpriteComponent.SetSprite` (`self.PaperSprite`) "/Game/gumboActors/soilSprites/wetSoilEmpty_Sprite.wetSoilEmpty_Sprite")))
    (elif (`self.hasSeeds`)
      (`PaperSpriteComponent.SetSprite` (`self.PaperSprite`) "/Game/gumboActors/soilSprites/drySoilPlanted_Sprite.drySoilPlanted_Sprite")
      (else
        (`PaperSpriteComponent.SetSprite` (`self.PaperSprite`) "/Game/gumboActors/soilSprites/drySoilEmpty_Sprite.drySoilEmpty_Sprite")))))

(fn `UserConstructionScript`)